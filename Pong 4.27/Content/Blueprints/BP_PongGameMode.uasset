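; Game mode for a Pong game that runs the match between the player and the AI, from serving balls to win or loss.
; On start it creates the HUD and picks a random serve direction along X.
; Score events update the HUD, then load WinScreen or LoseScreen at ten points, or serve again in a direction set by who scored.
; Each serve spawns a physics ball after a short delay, pauses, then sets its velocity.
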(event EventBeginPlay
  (bind _returnvalue (UserInterface|CreateWidget "/Game/Blueprints/BP_GameHUD.BP_GameHUD_C"))
  (bind _output_get (Variables|Default|SetGameHUDRef _returnvalue))
  (UserInterface|Viewport|AddtoViewport _output_get 0)
  (Variables|Default|SetDirection (Math|Float|Sign(Float) (Math|Random|RandomFloatinRange -1.0 1.0)))
  (Class|PongGameMode|SpawnNewBall))

(event EventIncreaseAIScore
  (bind _result (Math|Integer|IncrementInt (Variables|Default|GetAIScore))
    (:%20%20
      (Class|GameHUD|UpdateAIScore (Variables|Default|GetGameHUDRef) _result)
      (if (== (Variables|Default|GetAIScore) 10)
        (Game|OpenLevel(byName) "LoseScreen")
        (else
          (Variables|Default|SetDirection -1.0)
          (Class|PongGameMode|SpawnNewBall))))))

(event EventSpawnNewBall
  (Utilities|FlowControl|Delay 1.0)
  (bind _returnvalue (Game|SpawnActorfromClass "/Game/Blueprints/BP_Ball.BP_Ball_C" (Math|Transform|MakeTransform "0,10.000000, 0" "0, 0, 0" "1,1,1") "AlwaysSpawn" 0 0))
  (bind _output_get (Variables|Default|SetBallRef _returnvalue))
  (Utilities|FlowControl|Delay 0.5)
  (Physics|SetPhysicsLinearVelocity (Variables|/Script/Pong.Ball|GetSphere _output_get) (Math|Vector|MakeVector (* (Variables|Default|GetDirection) (Variables|Default|GetBallSpeed)) 0.0 0.0) false "None"))

(event EventIncreasePlayerScore
  (bind _result (Math|Integer|IncrementInt (Variables|Default|GetPlayerScore))
    (:%20%20
      (Class|GameHUD|UpdatePlayerScore (Variables|Default|GetGameHUDRef) _result)
      (if (== (Variables|Default|GetPlayerScore) 10)
        (Game|OpenLevel(byName) "WinScreen")
        (else
          (Variables|Default|SetDirection 1.0)
          (Class|PongGameMode|SpawnNewBall))))))

(fn ConstructionScript)